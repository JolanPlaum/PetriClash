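; BP_LevelTile is a board tile that holds one player's BP_Bacteria and can be captured by neighboring bacteria.
; It can spawn a starting bacteria, and Sprayed heals its occupant for the matching player.
; CheckTakeover sums weighted neighbor health per rival player, spawning the strongest's bacteria when it exceeds the tile's threshold.
; UpdateTileData destroys the old occupant, promotes the newcomer after a timer, and otherwise drains health until death.
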(event `self.ReceiveBeginPlay`
  (if (!= (`self.StartPlayerID`) -1)
    (bind _returnvalue (`|SpawnActorFromClass` "/Game/Blueprints/BP_Bacteria.BP_Bacteria_C" (`self.GetTransform`) "Undefined" "MultiplyWithRoot" null (`self.StartPlayerID`) 100.0 null))
    (set `self.NewBacteria` _returnvalue)))

(fn `CheckTakeover`
  (locals (OwningPlayerID :type Integer :default 0) (HealthNeeded :type "Float (double-precision)" :default 0.0) (PlayerTakeoverHealths :type "Array of Float (double-precision)"))
  (bind _playertakeoverhealths (`local.PlayerTakeoverHealths`))
  (bind _returnvalue (`KismetSystemLibrary.IsValid` (`self.OwningBacteria`)))
  (bind (_indexofmaxvalue _maxvalue) (`KismetMathLibrary.MaxOfFloatArray` (`local.PlayerTakeoverHealths`)))
  (if (not (`self.IsBeingTakenover`))
    (`|ExecutionSequence`
      (:`then_0`
        ;[1 1 1] Set function variables based on whether this tile is empty or not
        (set `local.OwningPlayerID` (select `bool` _returnvalue :`false` -1 :`true` (`local.OwningPlayerID`)))
        (if _returnvalue
          (set `local.HealthNeeded` (`/Game/Blueprints/BP_Bacteria.GetTakeoverHealthNeeded` (`self.OwningBacteria`)))
          (else
            (set `local.HealthNeeded` (`self.TakeoverHealthNeeded`))))
        (bind _asbp_multiplayer_cursor (cast `/Game/Blueprints/BP_MultiplayerCursor` (`GameplayStatics.GetGameMode`)))
        (`KismetArrayLibrary.Array_Resize` (`local.PlayerTakeoverHealths`) (`/Game/Blueprints/BP_MultiplayerCursor.PlayerCount` _asbp_multiplayer_cursor)))
      (:`then_1`
        (for _array_element (`self.SurroundingTiles`)
          (`/Engine/EditorBlueprintResources/StandardMacros.IsValid` (break `/Game/Data/STileConnection` _array_element) ; Is the connected tile valid
            (:`Is Valid`
              (bind _owningbacteria (`/Game/Blueprints/BP_LevelTile.OwningBacteria` (break `/Game/Data/STileConnection` _array_element)))
              (`/Engine/EditorBlueprintResources/StandardMacros.IsValid` _owningbacteria ; Is the connected tile taken
                (:`Is Valid`
                  (bind _playerid (`/Game/Blueprints/BP_Bacteria.PlayerID` _owningbacteria))
                  (if (!= (`local.OwningPlayerID`) _playerid)
                    (`KismetArrayLibrary.Array_Set` _playertakeoverhealths _playerid (+ (`|GetArrayItem` _playertakeoverhealths _playerid) (* (`/Game/Blueprints/BP_Bacteria.Health` _owningbacteria) (`.Weight_5_0D6CA4D448B21D17A84963B346CFFBDB` (break `/Game/Data/STileConnection` _array_element)))))))))))
        (if (> _maxvalue (`local.HealthNeeded`))
          (bind _returnvalue_2 (`|SpawnActorFromClass` "/Game/Blueprints/BP_Bacteria.BP_Bacteria_C" (`self.GetTransform`) "Undefined" "MultiplyWithRoot" null _indexofmaxvalue (/ _maxvalue 4.0) null))
          (set `self.NewBacteria` _returnvalue_2)
          (set `self.TakeoverTimer` (`self.TakeoverTime`)))))))

(fn `IsBeingTakenover`
  (returns (Result :type Boolean))
  (return (> (`self.TakeoverTimer`) 0.0)))

(fn `Sprayed`
  (params (`Player ID` :type Integer :default -1) (Strength :type "Float (double-precision)"))
  (bind _owningbacteria (`self.OwningBacteria`))
  (`/Engine/EditorBlueprintResources/StandardMacros.IsValid` _owningbacteria
    (:`Is Valid`
      (if (== `Player ID` (`/Game/Blueprints/BP_Bacteria.PlayerID` _owningbacteria))
        (`/Game/Blueprints/BP_Bacteria.HealHealthPercentage` (`self.OwningBacteria`) (`local.Strength`))))))

(fn `UpdateTileData`
  (params (DeltaSeconds :type "Float (double-precision)"))
  (bind _owningbacteria (`self.OwningBacteria`))
  (bind _owningbacteria_2 (`self.OwningBacteria`))
  (if (or (`self.IsBeingTakenover`) (`KismetSystemLibrary.IsValid` (`self.NewBacteria`)))
    (`/Engine/EditorBlueprintResources/StandardMacros.IsValid` _owningbacteria_2
      (:`Is Valid`
        (`self.K2_DestroyActor` _owningbacteria_2)
        (set `self.OwningBacteria` null))
      (:`Is Not Valid`
        (bind _output_get (set `self.TakeoverTimer` (- (`self.TakeoverTimer`) (`local.DeltaSeconds`))))
        (if (<= _output_get 0.0)
          (set `self.OwningBacteria` (`self.NewBacteria`))
          (set `self.NewBacteria` null))))
    (else
      (`/Engine/EditorBlueprintResources/StandardMacros.IsValid` _owningbacteria ; Only update health if there's a bacteria
        (:`Is Valid`
          (bind _output_get_2 (set `/Game/Blueprints/BP_Bacteria.Health` (- (`/Game/Blueprints/BP_Bacteria.Health` _owningbacteria) (`KismetMathLibrary.Abs` (* (`/Game/Blueprints/BP_Bacteria.GetHealthLostPerSecond` _owningbacteria) (`local.DeltaSeconds`)))) _owningbacteria))
          (if (<= _output_get_2 0.0)
            (`self.K2_DestroyActor` (`self.OwningBacteria`))
            (set `self.OwningBacteria` null)))))))

(fn `UserConstructionScript`)