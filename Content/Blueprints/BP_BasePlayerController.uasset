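; Base player controller that moves the pawn's aim cursor and lets two local players share one keyboard.
; WASD and arrow key presses and releases add opposite offsets to InputKeyboardDirection on player controller 0 or 1 respectively, whichever controller receives the key.
; Tick passes the normalized direction to BP_BasePlayerPawn's MoveAimCursor, which IA_MoveAim also feeds directly.
; The IA_DropWater handler is empty.
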(event `self.ReceiveTick`
  (params (DeltaSeconds :type "Float (single-precision)"))
  (if (not (`KismetMathLibrary.IsNearlyZero2D` (`self.InputKeyboardDirection`)))
    (bind _asbp_base_player_pawn (cast `/Game/Blueprints/BP_BasePlayerPawn` (`self.K2_GetPawn`)))
    (`/Game/Blueprints/BP_BasePlayerPawn.MoveAimCursor` _asbp_base_player_pawn (`KismetMathLibrary.NormalSafe2D` (`self.InputKeyboardDirection`) 0.001))))

(event `EnhancedInput|/Game/Input/IA_MoveAim`
  (params (ActionValue :type "Vector2D Structure") (ElapsedSeconds :type "Float (double-precision)") (TriggeredSeconds :type "Float (double-precision)") (InputAction :type "InputAction Object Reference" :default "/Game/Input/IA_MoveAim.IA_MoveAim"))
  (:`Triggered`
    (bind _asbp_base_player_pawn (cast `/Game/Blueprints/BP_BasePlayerPawn` (`self.K2_GetPawn`)))
    (`/Game/Blueprints/BP_BasePlayerPawn.MoveAimCursor` _asbp_base_player_pawn ActionValue)))

(event `EnhancedInput|/Game/Input/IA_DropWater`
  (params (ActionValue :type Boolean) (ElapsedSeconds :type "Float (double-precision)") (TriggeredSeconds :type "Float (double-precision)") (InputAction :type "InputAction Object Reference" :default "/Game/Input/IA_DropWater.IA_DropWater")))

(event `Key|Up`
  (params (Key :type "Key Structure"))
  (:`Pressed`
    (`self.HandleKeyboardInput` 0.0 1.0))
  (:`Released`
    (`self.HandleKeyboardInput` 0.0 -1.0)))

(event `Key|W`
  (params (Key :type "Key Structure"))
  (:`Pressed`
    (`self.HandleKeyboardInput` 0.0 1.0 true))
  (:`Released`
    (`self.HandleKeyboardInput` 0.0 -1.0 true)))

(event `Key|Down`
  (params (Key :type "Key Structure"))
  (:`Pressed`
    (`self.HandleKeyboardInput` 0.0 -1.0))
  (:`Released`
    (`self.HandleKeyboardInput` 0.0 1.0)))

(event `Key|S`
  (params (Key :type "Key Structure"))
  (:`Pressed`
    (`self.HandleKeyboardInput` 0.0 -1.0 true))
  (:`Released`
    (`self.HandleKeyboardInput` 0.0 1.0 true)))

(event `Key|Right`
  (params (Key :type "Key Structure"))
  (:`Pressed`
    (`self.HandleKeyboardInput` 1.0))
  (:`Released`
    (`self.HandleKeyboardInput` -1.0)))

(event `Key|D`
  (params (Key :type "Key Structure"))
  (:`Pressed`
    (`self.HandleKeyboardInput` 1.0 0.0 true))
  (:`Released`
    (`self.HandleKeyboardInput` -1.0 0.0 true)))

(event `Key|Left`
  (params (Key :type "Key Structure"))
  (:`Pressed`
    (`self.HandleKeyboardInput` -1.0))
  (:`Released`
    (`self.HandleKeyboardInput` 1.0)))

(event `Key|A`
  (params (Key :type "Key Structure"))
  (:`Pressed`
    (`self.HandleKeyboardInput` -1.0 0.0 true))
  (:`Released`
    (`self.HandleKeyboardInput` 1.0 0.0 true)))

(fn `HandleKeyboardInput`
  (params (X :type "Float (double-precision)") (Y :type "Float (double-precision)") (Player1 :type Boolean))
  (bind _asbp_base_player_controller (cast `/Game/Blueprints/BP_BasePlayerController` (`GameplayStatics.GetPlayerController` (`KismetMathLibrary.Conv_BoolToInt` (not Player1)))))
  (`/Engine/EditorBlueprintResources/StandardMacros.IsValid` _asbp_base_player_controller
    (:`Is Valid`
      (set `/Game/Blueprints/BP_BasePlayerController.InputKeyboardDirection` (+ (`/Game/Blueprints/BP_BasePlayerController.InputKeyboardDirection` _asbp_base_player_controller) (`KismetMathLibrary.MakeVector2D` X Y)) _asbp_base_player_controller))))

(fn `UserConstructionScript`)