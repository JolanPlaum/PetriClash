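; Base player pawn that acts as an aim cursor, moved across the screen by directional input and placed in the world beneath it.
; MoveAimCursor stores a direction, which Tick integrates into a clamped, normalized screen position with aspect-ratio-corrected speed, then clears.
; Tick then flips Y, deprojects that position through player 0's camera and moves the pawn to the ray's Z=0 intersection, a step marked temporary.
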(event `self.ReceiveTick`
  (params (DeltaSeconds :type "Float (single-precision)"))
  (bind _returnvalue (`WidgetLayoutLibrary.GetViewportSize`))
  (bind (_returnvalue_x _returnvalue_y) (`KismetMathLibrary.BreakVector2D` (* (`self.AimSpeed`) _returnvalue)))
  (bind _output_get (set `self.ScreenPos` (`KismetMathLibrary.ClampAxes2D` (+ (`self.ScreenPos`) (* DeltaSeconds (`self.InputDirection`) (/ (`KismetMathLibrary.MakeVector2D` _returnvalue_y _returnvalue_x) (`KismetMathLibrary.GetMin2D` _returnvalue)))) 0.0 1.0)))
  ;[1 1 1] Reset Input
  (set `self.InputDirection` (0.0 0.0))
  (bind (_x _y) (`KismetMathLibrary.BreakVector2D` _output_get))
  (bind (_returnvalue_x_2 _returnvalue_y_2) (`KismetMathLibrary.BreakVector2D` (* (`KismetMathLibrary.MakeVector2D` _x (- 1.0 _y)) (`WidgetLayoutLibrary.GetViewportSize`))))
  (bind (_worldlocation _worlddirection) (`PlayerController.DeprojectScreenPositionToWorld` (`GameplayStatics.GetPlayerController` 0) _returnvalue_x_2 _returnvalue_y_2))
  (`self.K2_SetActorLocation` (- _worldlocation (* _worlddirection (/ (.z _worldlocation) (.z _worlddirection))))) ; TEMPORARY
)

(event `MoveAimCursor`
  (params (Direction :type "Vector2D Structure"))
  (set `self.InputDirection` Direction))

(fn `UserConstructionScript`)