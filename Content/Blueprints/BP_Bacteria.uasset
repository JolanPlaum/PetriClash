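; BP_Bacteria is a player-owned bacteria actor whose size shows its health, scaled every tick to its health fraction.
; On BeginPlay it sets the Player 1 mesh when PlayerID is zero and destroys itself if LifeSpan is not positive.
; Helper functions derive health loss per second and the takeover threshold, and apply clamped percentage healing.
; The graphs here never apply the health decay.
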(event `self.ReceiveBeginPlay`
  (`|ExecutionSequence`
    (:`then_0`
      (if (== (`self.PlayerID`) 0)
        (`StaticMeshComponent.SetStaticMesh` (`self.Sphere`) (select `int` (`self.PlayerID`) :`0` "/Game/Art/SM_Bacteria_PLayer_1.SM_Bacteria_PLayer_1" :`1` "/Game/Art/SM_Bacteria_PLayer_1.SM_Bacteria_PLayer_1" :!type "StaticMesh Object Reference"))))
    (:`then_1`
      (if (<= (`self.LifeSpan`) 0.0)
        (`self.K2_DestroyActor`)))))

(event `self.ReceiveTick`
  (params (DeltaSeconds :type "Float (single-precision)"))
  (`self.SetActorScale3D` (`KismetMathLibrary.Conv_DoubleToVector` (`self.GetHealthPercentage`))))

(fn `GetHealthLostPerSecond`
  (returns (HealthLost :type "Float (double-precision)"))
  (return (/ (`self.MaxHealth`) (`self.LifeSpan`))))

(fn `GetHealthPercentage`
  (returns (HealthPercentage :type "Float (double-precision)"))
  (return (/ (`self.Health`) (`self.MaxHealth`))))

(fn `GetTakeoverHealthNeeded`
  (returns (TakeoverHealthNeeded :type "Float (double-precision)"))
  (return (+ (`self.Health`) (`self.TakeoverHealthAddition`))))

(fn `HealHealthPercentage`
  (params (HealPercentage :type "Float (double-precision)"))
  (set `self.Health` (`KismetMathLibrary.FClamp` (+ (* HealPercentage (`self.MaxHealth`)) (`self.Health`)) 0.0 (`self.MaxHealth`))))

(fn `UserConstructionScript`)