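; BP_MultiplayerCursor sets up local multiplayer on a shared camera with a visible mouse cursor.
; On BeginPlay it loops over PlayerCount, reusing the first controller and creating the rest, then gives each IMC_Default input and a possessed BP_BasePlayerPawn spawned at the origin.
; It then points the first controller's view at BP_MainCamera and shows its cursor.
; Tick prints viewport scale and size on screen for debugging.
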(event `self.ReceiveBeginPlay`
  (`|ExecutionSequence`
    (:`then_0`
      (for _index (range (`self.PlayerCount`))
        (bind _returnvalue (`GameplayStatics.CreatePlayer` _index))
        (bind _returnvalue_2 (select `bool` (> _index 0) :`false` (`GameplayStatics.GetPlayerController` 0) :`true` _returnvalue))
        (`EnhancedInputSubsystemInterface.AddMappingContext` (pcsubsystem `EnhancedInputLocalPlayerSubsystem` _returnvalue_2) "/Game/Input/IMC_Default.IMC_Default" 0 (struct))
        (bind _returnvalue_3 (`|SpawnActorFromClass` "/Game/Blueprints/BP_BasePlayerPawn.BP_BasePlayerPawn_C" (`KismetMathLibrary.MakeTransform` (0.0 0.0 0.0)) "Undefined" "MultiplyWithRoot" null 0.25 null))
        (`Controller.Possess` _returnvalue_2 _returnvalue_3)))
    (:`then_1`
      ;[1 1 1] Set camera view
      (bind _returnvalue_4 (`GameplayStatics.GetActorOfClass` "/Game/Blueprints/BP_MainCamera.BP_MainCamera_C"))
      (`PlayerController.SetViewTargetWithBlend` (`GameplayStatics.GetPlayerController` 0) _returnvalue_4 0.0 "VTBlend_Linear" 0.0 false))
    (:`then_2`
      (set `PlayerController.bShowMouseCursor` true (`GameplayStatics.GetPlayerController` 0)))))

(event `self.ReceiveTick`
  (params (DeltaSeconds :type "Float (single-precision)"))
  (`KismetSystemLibrary.PrintString` (`KismetStringLibrary.Conv_DoubleToString` (`WidgetLayoutLibrary.GetViewportScale`)) true false (struct :`R` 1.0 :`B` 0.029831 :`A` 1.0) 0.0)
  (`KismetSystemLibrary.PrintString` (`KismetStringLibrary.Conv_Vector2dToString` (`WidgetLayoutLibrary.GetViewportSize`)) true false (struct :`R` 1.0 :`B` 0.029831 :`A` 1.0) 0.0))

(fn `UserConstructionScript`)