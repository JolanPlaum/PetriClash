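; Grid manager that indexes placed BP_LevelTile actors and drives their takeover simulation.
; On BeginPlay it derives tile size from actor scale and grid bounds from positions, then maps tiles into a flat row-major array that allows gaps.
; Each tile receives its eight-way neighbours as weighted connections, with diagonals scaled by a separate factor.
; Tick runs CheckTakeover on every tile before a second pass updates tile data.
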(event `self.ReceiveBeginPlay`
  (bind _outactors (`GameplayStatics.GetAllActorsOfClass` "/Game/Blueprints/BP_LevelTile.BP_LevelTile_C"))
  (`|ExecutionSequence`
    (:`then_0`
      ;[1 1 1] Calculate tile size
      (for _array_element _outactors
        (`/Engine/EditorBlueprintResources/StandardMacros.IsValid` _array_element
          (:`Is Valid`
            (bind (_returnvalue_x _returnvalue_y) (`KismetMathLibrary.BreakVector` (`Actor.GetActorScale3D` _array_element)))
            (if (`KismetMathLibrary.NearlyEqual_FloatFloat` _returnvalue_x _returnvalue_y)
              (set `self.TileSize` (* (`self.TileSize`) _returnvalue_x))
              (break)
              (else
                (`KismetSystemLibrary.PrintString` "WARNING: Level tiles were not scaled equally along X/Y axis!" true true (struct :`R` 1.0 :`A` 1.0) 10.0)))))))
    (:`then_1`
      (bind (_min _max) (`self.GetMinMaxPositions` _outactors))
      (bind _output_get (set `self.OriginOffset` _min))
      (bind (_returnvalue_x_2 _returnvalue_y_2) (`KismetMathLibrary.BreakVector` (/ (- _max _output_get) (`self.TileSize`))))
      (bind _result (`/Engine/EditorBlueprintResources/StandardMacros.IncrementInt` (`KismetMathLibrary.Round` _returnvalue_x_2))
        (:`  `
          (set `self.NrCols` _result)
          (bind _result_2 (`/Engine/EditorBlueprintResources/StandardMacros.IncrementInt` (`KismetMathLibrary.Round` _returnvalue_y_2))
            (:`  `
              (set `self.NrRows` _result_2))))))
    (:`then_2`
      (`KismetArrayLibrary.Array_Resize` (`self.Tiles`) (* (`self.NrCols`) (`self.NrRows`)))
      (for _array_element_2 _outactors
        (`KismetArrayLibrary.Array_Set` (`self.Tiles`) (`self.PositionToIndex` (`Actor.K2_GetActorLocation` _array_element_2)) _array_element_2)))
    (:`then_3`
      (for (_array_element_3 _array_index) (`self.Tiles`)
        (`/Engine/EditorBlueprintResources/StandardMacros.IsValid` _array_element_3
          (:`Is Valid`
            (bind _surroundingtiles (`self.GetSurroundingTiles` (`self.IndexToColumn` _array_index) (`self.IndexToRow` _array_index)))
            (set `/Game/Blueprints/BP_LevelTile.SurroundingTiles` _surroundingtiles _array_element_3)))))))

(event `self.ReceiveTick`
  (params (DeltaSeconds :type "Float (single-precision)"))
  (bind _tiles (`self.Tiles`))
  (`|ExecutionSequence`
    (:`then_0`
      (for _array_element _tiles
        (`/Engine/EditorBlueprintResources/StandardMacros.IsValid` _array_element
          (:`Is Valid`
            (`/Game/Blueprints/BP_LevelTile.CheckTakeover` _array_element)))))
    (:`then_1`
      (for _array_element_2 _tiles
        (`/Engine/EditorBlueprintResources/StandardMacros.IsValid` _array_element_2
          (:`Is Valid`
            (`/Game/Blueprints/BP_LevelTile.UpdateTileData` _array_element_2 DeltaSeconds)))))))

(fn `ColumnRowToIndex`
  (params (Column :type Integer) (Row :type Integer))
  (returns (Index :type Integer))
  (if (and (`KismetMathLibrary.InRange_IntInt` Column 0 (`self.NrCols`) true false) (`KismetMathLibrary.InRange_IntInt` Row 0 (`self.NrRows`) true false))
    (return (+ (`local.Column`) (* (`local.Row`) (`self.NrCols`))))
    (else
      (return -1))))

(fn `GetMinMaxPositions`
  (params (LevelTiles :type "Array of /Game/Blueprints/BP_LevelTile Object Reference"))
  (returns (Min :type "Vector Structure") (Max :type "Vector Structure"))
  (locals (TileLocationsX :type "Array of Float (double-precision)") (TileLocationsY :type "Array of Float (double-precision)") (TileLocationsZ :type "Array of Float (double-precision)"))
  (bind _returnvalue (`KismetArrayLibrary.Array_Length` LevelTiles))
  (`|ExecutionSequence`
    (:`then_0`
      (`KismetArrayLibrary.Array_Resize` (`local.TileLocationsX`) _returnvalue))
    (:`then_1`
      (`KismetArrayLibrary.Array_Resize` (`local.TileLocationsY`) _returnvalue))
    (:`then_2`
      (`KismetArrayLibrary.Array_Resize` (`local.TileLocationsZ`) _returnvalue))
    (:`then_3`
      (for (_array_element _array_index) LevelTiles
        (bind (_returnvalue_x _returnvalue_y _returnvalue_z) (`KismetMathLibrary.BreakVector` (`Actor.K2_GetActorLocation` _array_element)))
        (`KismetArrayLibrary.Array_Set` (`local.TileLocationsX`) _array_index _returnvalue_x)
        (`KismetArrayLibrary.Array_Set` (`local.TileLocationsY`) _array_index _returnvalue_y)
        (`KismetArrayLibrary.Array_Set` (`local.TileLocationsZ`) _array_index _returnvalue_z))
      (return (`KismetMathLibrary.MakeVector` (`.MinValue` (`KismetMathLibrary.MinOfFloatArray` (`local.TileLocationsX`))) (`.MinValue` (`KismetMathLibrary.MinOfFloatArray` (`local.TileLocationsY`))) (`.MinValue` (`KismetMathLibrary.MinOfFloatArray` (`local.TileLocationsZ`)))) (`KismetMathLibrary.MakeVector` (`.MaxValue` (`KismetMathLibrary.MaxOfFloatArray` (`local.TileLocationsX`))) (`.MaxValue` (`KismetMathLibrary.MaxOfFloatArray` (`local.TileLocationsY`))) (`.MaxValue` (`KismetMathLibrary.MaxOfFloatArray` (`local.TileLocationsZ`))))))))

(fn `GetSurroundingTiles`
  (params (Column :type Integer) (Row :type Integer))
  (returns (SurroundingTiles :type "Array of /Game/Data/STileConnection Structure"))
  (locals (TileConnections :type "Array of /Game/Data/STileConnection Structure") (DiagonalLineWeight :type "Float (double-precision)" :default 0.707107))
  (bind _maxconnectionweight (`self.MaxConnectionWeight`))
  (for _index (range (- Column 1) (+ (+ Column 1) 1))
    (for _index_2 (range (- Row 1) (+ (+ Row 1) 1))
      (bind _index_3 (`self.ColumnRowToIndex` _index _index_2))
      (if (!= _index_3 -1)
        (bind _output (`|GetArrayItem` (`self.Tiles`) _index_3))
        (`/Engine/EditorBlueprintResources/StandardMacros.IsValid` _output ; Check if there is a tile or obstacle
          (:`Is Valid`
            (if (!= _index_3 (`self.ColumnRowToIndex` (`local.Column`) (`local.Row`)))
              (`KismetArrayLibrary.Array_Add` (`local.TileConnections`) (make `/Game/Data/STileConnection` _output (select `bool` (or (== _index (`local.Column`)) (== _index_2 (`local.Row`))) :`false` (* (`local.DiagonalLineWeight`) _maxconnectionweight) :`true` _maxconnectionweight)))))))))
  (return (`local.TileConnections`)))

(fn `IndexToColumn`
  (params (Index :type Integer))
  (returns (Column :type Integer))
  (if (`KismetArrayLibrary.Array_IsValidIndex` (`self.Tiles`) Index)
    (return (mod Index (`self.NrCols`)))
    (else
      (return -1024))))

(fn `IndexToRow`
  (params (Index :type Integer))
  (returns (Row :type Integer))
  (if (`KismetArrayLibrary.Array_IsValidIndex` (`self.Tiles`) Index)
    (return (/ Index (`self.NrCols`)))
    (else
      (return -1024))))

(fn `PositionToColumnRow`
  (params (Location :type "Vector Structure"))
  (returns (Column :type Integer) (Row :type Integer))
  (bind (_returnvalue_x _returnvalue_y) (`KismetMathLibrary.BreakVector` (/ (- Location (`self.OriginOffset`)) (`self.TileSize`))))
  (return (`KismetMathLibrary.Round` _returnvalue_x) (`KismetMathLibrary.Round` _returnvalue_y)))

(fn `PositionToIndex`
  (params (Location :type "Vector Structure"))
  (returns (Index :type Integer))
  (bind (_column _row) (`self.PositionToColumnRow` Location))
  (return (`self.ColumnRowToIndex` _column _row)))